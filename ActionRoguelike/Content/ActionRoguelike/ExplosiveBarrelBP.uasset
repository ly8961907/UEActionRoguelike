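; Explosive barrel actor that blows up on a short fuse and damages actors it collides with.
; On BeginPlay the authority starts a one-shot timer that calls MulticastExplode to fire the RadialForce impulse, then destroys the actor.
; Separately, each mesh hit fires the impulse and subtracts health through the other actor's SAttributeComponent, without destroying the barrel or checking authority.
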(event OnComponentHit(StaticMesh)
  (params (HitComponent :type Primitive%20Component%20Object%20Reference) (OtherActor :type Actor%20Object%20Reference) (OtherComp :type Primitive%20Component%20Object%20Reference) (NormalImpulse :type Vector :default "0, 0, 0") (Hit :type Hit%20Result%20Structure%20%28by%20ref%29))
  (bind _returnvalue (Actor|GetComponentbyClass OtherActor "/Script/ActionRoguelike.SAttributeComponent"))
  (Utilities|IsValid OtherActor
    (:Is%20Valid
      (Class|RadialForceComponent|FireImpulse (Variables|Default|GetRadialForce))
      (Utilities|IsValid _returnvalue
        (:Is%20Valid
          (Class|SAttributeComponent|ApplyHealthChange _returnvalue 0 -2e+01))))))

(event Custom|Explode
  (CallFunction|MulticastExplode)
  (Actor|DestroyActor))

(event Custom|MulticastExplode
  (Class|RadialForceComponent|FireImpulse (Variables|Default|GetRadialForce)))

(event EventBeginPlay
  (if (Ability|HasAuthority)
    (Utilities|Time|SetTimerbyEvent (delegate Custom|Explode) 4.0)))

(fn ConstructionScript)